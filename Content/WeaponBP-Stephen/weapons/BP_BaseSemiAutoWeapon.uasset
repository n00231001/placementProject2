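; Base semi-automatic weapon Blueprint that extends its parent's Shoot event with single-shot firing.
; After the parent call, if CanShoot is true, it creates a shot trace over Range and applies pitch input to the player character as recoil.
; It then starts a FireRate timer bound to ResetShot, which is empty here, and nothing in this graph changes CanShoot.
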(event Custom|ResetShot)

(event EventShoot
  (|CallParentFunction)
  (if (Variables|Default|GetCanShoot)
    (CallFunction|CreateShotTrace (Variables|Default|GetRange))
    (Pawn|Input|AddControllerPitchInput (Variables|Default|GetPlayerCharacter) -0.2)
    (Utilities|Time|SetTimerbyEvent (delegate Custom|ResetShot) (Variables|Default|GetFireRate))))

(fn ConstructionScript
  (|CallParentFunction))