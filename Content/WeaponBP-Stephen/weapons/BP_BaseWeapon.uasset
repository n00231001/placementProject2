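; Base weapon Blueprint with empty Shoot and EndShoot events and a shared hitscan CreateShotTrace event.
; Each shot decrements magazine ammo, updates the cached first-person character, plays fire effects, then line-traces from ShootArrow to damage pawns or physics bodies with blood splats.
; When the count hits zero, it clicks instead of firing, blocks shooting and automatically refills after a delay, with no reserve ammo tracked.
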(event Custom|CreateShotTrace
  (params (Range :type Float%20%28double-precision%29))
  (bind _shootarrow (Variables|Default|GetShootArrow))
  (bind _returnvalue (Transformation|GetWorldLocation _shootarrow))
  (bind _output_get (Variables|Default|SetCurrentMagAmmo (Math|Integer|Clamp(Integer) (- (Variables|Default|GetCurrentMagAmmo) 1) 0 (Variables|Default|GetMaxMagAmmo))))
  (Default|UpdateAmmo (Variables|Default|GetPlayerCharacter) _output_get)
  (if (<= _output_get 0)
    (Utilities|FlowControl|Delay 0.2)
    (Audio|PlaySoundatLocation "/Game/InterfaceAndItemSounds/WAV/Click_09_wav.Click_09_wav" "0, 0, 0" "0, 0, 0" 1.0 1.0 0.0 0 0 0 0)
    (Variables|Default|SetCanShoot false)
    (Utilities|FlowControl|Delay 2.0)
    (Variables|Default|SetCurrentMagAmmo (Variables|Default|GetMaxMagAmmo))
    (Variables|Default|SetCanShoot true)
    (else
      (Audio|PlaySoundatLocation (Variables|Default|GetFireSound) "0, 0, 0" "0, 0, 0" 1.0 1.0 0.0 0 0 0 0)
      (Effects|SpawnEmitterAttached "/Game/Realistic_Starter_VFX_Pack_Vol2/Particles/Explosion/P_Explosion_Big_A.P_Explosion_Big_A" _shootarrow "None" "0, 0, 0" "0, 0, 0" "0.050000,0.050000,0.050000")
      (bind (_outhit _returnvalue_2) (Collision|LineTraceForObjects _returnvalue (+ _returnvalue (* (Math|Vector|GetForwardVector (Transformation|GetWorldRotation _shootarrow)) Range)) (Utilities|Array|MakeArray "ObjectTypeQuery3" "ObjectTypeQuery4") false 0 "None"))
      (if _returnvalue_2
        (bind _array_element (Utilities|Array|ForEachLoopwithBreak (Utilities|Array|MakeArray _outhit))
          (:LoopBody
            (Effects|SpawnEmitteratLocation "/Game/Realistic_Starter_VFX_Pack_Vol2/Particles/Blood/P_Blood_Splat_Cone.P_Blood_Splat_Cone" (.Location (Collision|BreakHitResult _array_element)))
            (Game|Damage|ApplyDamage (.HitActor (Collision|BreakHitResult _array_element)) (Variables|Default|GetDamage) 0 0)))))))

(event Custom|Shoot)

(event Custom|EndShoot)

(event EventBeginPlay
  (bind _asbp_first_person_character (Utilities|Casting|CastToBP_FirstPersonCharacter (Game|GetPlayerCharacter 0)))
  (Variables|Default|SetPlayerCharacter _asbp_first_person_character))

(fn ConstructionScript)