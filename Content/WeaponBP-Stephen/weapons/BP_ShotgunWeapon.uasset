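; Shotgun weapon Blueprint that extends a parent weapon's Shoot event with its own firing effects.
; After the parent call, if CanShoot is true it attaches a smoke burst at ShootArrow, creates a shot trace over Range and kicks the player's pitch for recoil.
; It then sets a FireRate-long timer to ResetShot, which has no logic in this Blueprint.
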(event Custom|ResetShot)

(event EventShoot
  (|CallParentFunction)
  (if (Variables|Default|GetCanShoot)
    (Effects|SpawnEmitterAttached "/Game/Realistic_Starter_VFX_Pack_Vol2/Particles/Explosion/P_Explosion_Smoke.P_Explosion_Smoke" (Variables|Default|GetShootArrow) "None" "0, 0, 0" "0, 0, 0" "0.500000,0.500000,0.500000")
    (CallFunction|CreateShotTrace (Variables|Default|GetRange))
    (Pawn|Input|AddControllerPitchInput (Variables|Default|GetPlayerCharacter) -1.0)
    (Utilities|Time|SetTimerbyEvent (delegate Custom|ResetShot) (Variables|Default|GetFireRate))))

(fn ConstructionScript
  (|CallParentFunction))