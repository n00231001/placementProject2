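; BP_UltimateWeapon is a full-auto child weapon that the player holds until its magazine runs dry.
; Shoot starts a looping FireRate timer that EndShoot clears; each tick traces a shot, adds pitch recoil and plays a pistol sound at world origin.
; When magazine ammo is empty, it resets the first-person character's KillCount and has it spawn the base semi-auto weapon.
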(event Custom|FullAutoShoot
  (CallFunction|CreateShotTrace (Variables|Default|GetRange))
  (Pawn|Input|AddControllerPitchInput (Variables|Default|GetPlayerCharacter) -0.1)
  (Audio|PlaySoundatLocation "/Game/FreeGunSounds/Wav/Pistol/WAV_PistolShot01.WAV_PistolShot01" "0, 0, 0" "0, 0, 0" 1.0 1.0 0.0 0 0 0 0)
  (if (<= (Variables|Default|GetCurrentMagAmmo) 0)
    (bind _asbp_first_person_character (Utilities|Casting|CastToBP_FirstPersonCharacter (Game|GetPlayerCharacter 0)))
    (Variables|/Game/FirstPerson/Blueprints/BP_FirstPersonCharacter.BP_FirstPersonCharacter_C|SetKillCount _asbp_first_person_character 0)
    (Default|SpawnWeapon _asbp_first_person_character "/Game/WeaponBP-Stephen/weapons/BP_BaseSemiAutoWeapon.BP_BaseSemiAutoWeapon_C")))

(event EventShoot
  (|CallParentFunction)
  (bind _returnvalue (Utilities|Time|SetTimerbyEvent (delegate Custom|FullAutoShoot) (Variables|Default|GetFireRate) true))
  (Variables|Default|SetTimer _returnvalue))

(event EventEndShoot
  (|CallParentFunction)
  (Utilities|Time|ClearandInvalidateTimerbyHandle (Variables|Default|GetTimer)))

(fn ConstructionScript
  (|CallParentFunction))