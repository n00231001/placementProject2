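; Trigger actor for combat arena 6 that plays the CombatArena6 level sequence when the first-person character enters its box.
; The overlap creates and stores the sequence player, then plays it forward once.
; Tick polls the player character's KillCount and plays the sequence in reverse once it reaches the hard-coded threshold.
; A debug key also triggers the reverse playback.
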(event OnComponentBeginOverlap(Box)
  (params (OverlappedComponent :type Primitive%20Component%20Object%20Reference) (OtherActor :type Actor%20Object%20Reference) (OtherComp :type Primitive%20Component%20Object%20Reference) (OtherBodyIndex :type Integer) (bFromSweep :type Boolean) (SweepResult :type Hit%20Result%20Structure%20%28by%20ref%29))
  (Utilities|Casting|CastToBP_FirstPersonCharacter OtherActor)
  (Utilities|FlowControl|DoOnce false
    (:Completed
      (bind _returnvalue (Sequencer|Player|CreateLevelSequencePlayer "/Game/Sequencers/combatArena6.combatArena6"))
      (Variables|Default|SetMySequencePlay _returnvalue)
      (Sequencer|Player|Play _returnvalue :!class /Script/MovieScene.MovieSceneSequencePlayer))))

(event EventBeginPlay)

(event Collision|EventActorBeginOverlap
  (params (OtherActor :type Actor%20Object%20Reference)))

(event EventTick
  (params (DeltaSeconds :type Float%20%28single-precision%29))
  (bind _asbp_first_person_character (Utilities|Casting|CastToBP_FirstPersonCharacter (Game|GetPlayerCharacter 0)))
  (if (>= (Variables|/Game/FirstPerson/Blueprints/BP_FirstPersonCharacter.BP_FirstPersonCharacter_C|GetKillCount _asbp_first_person_character) 100)
    (Utilities|FlowControl|DoOnce false
      (:Completed
        (Class|MovieSceneSequencePlayer|PlayReverse (Variables|Default|GetMySequencePlay))))))

(event Input|KeyboardEvents|DebugKey2
  (params (Key :type Key%20Structure :default "None") (ActionValue :type Input%20Action%20Value%20Structure))
  (:Pressed
    (Class|MovieSceneSequencePlayer|PlayReverse (stale OnComponentBeginOverlap(Box) _returnvalue))))

(fn ConstructionScript)