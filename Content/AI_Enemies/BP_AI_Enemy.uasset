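; BP_AI_Enemy is an AI enemy that turns to face the first-person player when it sees them.
; PawnSensing's OnSeePawn casts to BP_FirstPersonCharacter and snaps the enemy's rotation toward that character's location.
; The following CanAttack check leads nowhere, leaving the damage and cooldown chain disconnected.
; A SpawnProjectileLocation component is referenced only by an unused node, so no attack occurs here.
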(event OnSeePawn(PawnSensing)
  (params (Pawn :type Pawn%20Object%20Reference))
  (bind _asbp_first_person_character (Utilities|Casting|CastToBP_FirstPersonCharacter Pawn))
  (Transformation|SetActorRotation (Math|Rotator|FindRelativeLookatRotation (Math|Conversions|ToTransform(Vector) (Transformation|GetActorLocation)) (Transformation|GetActorLocation _asbp_first_person_character)))
  (if (Variables|Default|GetCanAttack?)
    _))

(event EventBeginPlay)

(event Collision|EventActorBeginOverlap
  (params (OtherActor :type Actor%20Object%20Reference)))

(event EventTick
  (params (DeltaSeconds :type Float%20%28single-precision%29)))

(fn ConstructionScript)