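; BP_health is a health and shield Blueprint, with only the health math implemented so far.
; GainHealth and TakeHealth clamp CurrentHealth between zero and MaxHealth, and TakeHealth calls Death when HasHealth returns false.
; HasHealth and HasShield contain non-zero comparisons that are left unused.
; Death, GainShield, TakeShield, HealthUpdate and the event graph are empty stubs.
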(event EventBeginPlay)

(event Collision|EventActorBeginOverlap
  (params (OtherActor :type Actor%20Object%20Reference)))

(event EventTick
  (params (DeltaSeconds :type Float%20%28single-precision%29)))

(fn ConstructionScript)

(fn GainHealth
  (params (Health :type Float%20%28double-precision%29))
  (bind _output_get (Variables|Default|SetCurrent%20Health (Math|Float|Clamp(Float) (+ Health (Variables|Default|GetCurrent%20Health)) 0.0 (Variables|Default|GetMax%20Health))))
  (return _output_get))

(fn TakeHealth
  (params (Damage :type Float%20%28double-precision%29))
  (Variables|Default|SetCurrent%20Health (Math|Float|Clamp(Float) (- (Variables|Default|GetCurrent%20Health) Damage) 0.0 (Variables|Default|GetMax%20Health)))
  (if (not (Utilities|HasHealth))
    (CallFunction|Death)))

(fn Death)

(fn GainShield)

(fn TakeShield)

(fn HealthUpdate)