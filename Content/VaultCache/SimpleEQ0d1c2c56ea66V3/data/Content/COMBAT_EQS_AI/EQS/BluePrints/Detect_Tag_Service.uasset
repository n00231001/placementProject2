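; Behavior Tree service that tells teammates from enemies by team tag and drives AI shooting and cover.
; Each tick it sphere-traces from the pawn to the focus actor, storing a hit character in the TeamPlayer or TargetActor Blackboard key.
; An enemy hit triggers Shoot and starts timers that clear inCombat and move the AI to the CoverMove location.
; When the move finishes, it sets InCover and calls EnterCover.
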(event Custom|MoveToCoverCrouch
  ;[1 0.8187 0.07785] Get To Cover After 4 Seconds Of Fighting
  ;;[0.4235 1 0.3365] If Enemy Detected Is True Then Move To Coordinated From Cover EQS
  (if (Variables|Default|GetEnemyDetected)
    (AI|AIMoveTo (Variables|References|GetAI%20Controller%20Ref) (Class|BTFunctionLibrary|GetBlackboardValueasVector (Variables|Blackboard|GetCoverMove)) 0 -1.0 "Default" "Default" true true
      (:OnMoveFinished
        ;;[1 0.3664 0.8557] Tells AI To Move To Cover And Set CoverBB Value True
        (bind _asbase_ai_character (Utilities|Casting|CastToBase_AI_Character (Variables|References|GetPawn%20Ref)))
        (Class|BTFunctionLibrary|SetBlackboardValueasBool (Variables|Blackboard|GetInCover) true)
        (Default|EnterCover _asbase_ai_character)))))

(event Custom|Set%20inCombat%20To%20False
  (bind _ai_bb_ref (Variables|Default|GetAI_BB%20Ref))
  ;[0.6637 1 0.9093] Ensures that inCombat is set to false when not shooting. Shooting will set it to true.
  (Utilities|IsValid _ai_bb_ref
    (:Is%20Valid
      (AI|Components|Blackboard|SetValueasBool _ai_bb_ref (Utilities|Name|MakeLiteralName "inCombat") false))))

(event Custom|Run%20inCombat%20Bool%20Event
  ;[0.004992 0.2656 0] Detect Enemy And Shoot
  ;;[1 0.1543 0.1244] Waits a certain amount of time before calling the event to set inCombat to False.
  (CallFunction|SetinCombattoFalse))

(event Custom|Start%20MoveToCover
  ;[0.004992 0.2656 0] Detect Enemy And Shoot
  ;;[0.3728 1 0.9502] Starts The Custom Event To Get Cover
  (CallFunction|MovetoCoverCrouch))

(event EventReceiveTickAI
  (params (OwnerController :type AI%20Controller%20Object%20Reference) (ControlledPawn :type Pawn%20Object%20Reference) (DeltaSeconds :type Float%20%28single-precision%29))
  (bind _as_base_character (Variables|References|GetAs%20Base%20Character))
  ;[0.004992 0.2656 0] Detect Enemy And Shoot
  (Variables|References|SetAI%20Controller%20Ref OwnerController)
  (Variables|References|SetPawn%20Ref ControlledPawn)
  (Utilities|IsValid (Class|AIController|GetFocusActor (Variables|References|GetAI%20Controller%20Ref))
    (:Is%20Valid
      (Utilities|IsValid (Variables|References|GetPawn%20Ref)
        (:Is%20Valid
          ;;[0.49 1 0.4779] Creates Sphere, based on Radius size, for detecting enemies
          (bind (_outhit _returnvalue) (Collision|SphereTraceByChannel (Transformation|GetActorLocation (Variables|References|GetPawn%20Ref)) (Transformation|GetActorLocation (Class|AIController|GetFocusActor (Variables|References|GetAI%20Controller%20Ref))) 5.0 "TraceTypeQuery2" false (Utilities|Array|MakeArray (Variables|References|GetAs%20Base%20Character)) "None"))
          (if _returnvalue
            ;;[0.06772 0.7891 1] Gets Detected Player's Team Tag
            (bind _asbase_character (Utilities|Casting|CastToBase_Character (.HitActor (Collision|BreakHitResult _outhit))))
            (if (== (Variables|Blackboard|GetThis%20AI%20Team%20Tag) (Variables|/Game/COMBAT_EQS_AI/Characters/ParentChar/Base_Character.Base_Character_C|GetTeamTag _asbase_character))
              ;;;[0.1296 0 1] Sets Team BB Key If Teamate
              (Class|BTFunctionLibrary|SetBlackboardValueasObject (Variables|Blackboard|GetTeamPlayer) _asbase_character)
              (else
                ;;;[1 0.04544 0] Sets Target BB Key If Enemy
                (Class|BTFunctionLibrary|SetBlackboardValueasObject (Variables|Blackboard|GetTargetActor) _asbase_character)
                (Variables|Default|SetEnemyDetected true)
                (Utilities|Time|SetTimerbyEvent (delegate Custom|Start%20MoveToCover) 4.0)
                ;;[1 0.982 0.3033] Start To Shoot. Carries Over Enemy Tag
                (Utilities|IsValid _as_base_character
                  (:Is%20Valid
                    (bind _asbase_ai_character (Utilities|Casting|CastToBase_AI_Character _as_base_character))
                    (Default|Shoot _asbase_ai_character)
                    ;;[1 0.1543 0.1244] Waits a certain amount of time before calling the event to set inCombat to False.
                    (Utilities|Time|SetTimerbyEvent (delegate Custom|Run%20inCombat%20Bool%20Event) 2.5)))))))))))

(event EventReceiveActivationAI
  (params (OwnerController :type AI%20Controller%20Object%20Reference) (ControlledPawn :type Pawn%20Object%20Reference))
  ;[0.08647 0.2126 0.2812] Gets The Team Tag Of Current AI
  (bind _asbase_character (Utilities|Casting|CastToBase_Character ControlledPawn))
  (bind _output_get (Variables|References|SetAs%20Base%20Character _asbase_character))
  (Variables|Blackboard|SetThis%20AI%20Team%20Tag (Variables|/Game/COMBAT_EQS_AI/Characters/ParentChar/Base_Character.Base_Character_C|GetTeamTag _output_get)))