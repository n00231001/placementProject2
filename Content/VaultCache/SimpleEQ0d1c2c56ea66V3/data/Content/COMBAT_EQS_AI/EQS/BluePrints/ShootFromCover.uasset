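; Behavior tree task that makes an enemy AI character pop up from cover and fire, used by the cover behavior tree.
; On execute it uncrouches the Base_AI_Character, calls Shoot once, and starts a random-length timer that crouches it again and finishes the task successfully.
; While active, its tick sets the AI controller's focal point to the player pawn's location for aiming.
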(event Custom|StopShooting
  ;[0.5784 1 0.5481] Stop shooting and crouch
  (Character|Crouch (Variables|Default|GetEnemyPawn))
  (AI|BehaviorTree|FinishExecute true))

(event EventReceiveExecuteAI
  (params (OwnerController :type AI%20Controller%20Object%20Reference) (ControlledPawn :type Pawn%20Object%20Reference))
  ;[0.3184 1 0.5592] Stand up as soon as this event is called in the AI_BT_COVER
  (bind _asbase_ai_character (Utilities|Casting|CastToBase_AI_Character ControlledPawn))
  (bind _output_get (Variables|Default|SetEnemyPawn _asbase_ai_character))
  (Character|UnCrouch _output_get)
  ;[1 0.1382 0.5198] Once standing, start shooting
  (Default|Shoot (Variables|Default|GetEnemyPawn))
  ;[1 0.9743 0.3585] Shoot for random time within range of 2 floats. After random time, call the next event StopShooting
  (Utilities|Time|SetTimerbyEvent (delegate Custom|StopShooting) (Math|Random|RandomFloatinRange 2.0 1e+01)))

(event EventReceiveTickAI
  (params (OwnerController :type AI%20Controller%20Object%20Reference) (ControlledPawn :type Pawn%20Object%20Reference) (DeltaSeconds :type Float%20%28single-precision%29))
  (bind _returnvalue (Game|Player|GetPlayerPawn 0))
  ;[0.8629 0.4846 1] Look at the pawn when shooting from character for aiming
  (Utilities|IsValid _returnvalue
    (:Is%20Valid
      (AI|SetFocalPoint OwnerController (Transformation|GetActorLocation _returnvalue)))))