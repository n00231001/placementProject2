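; Behavior tree service that makes an AI character shoot at enemies toward its focus actor.
; Each tick it sphere-traces from the pawn to the controller's focus actor, casts the hit to Base_Character and calls Shoot when the team tags differ.
; An event that moves the AI to a blackboard cover location and crouches it is left unwired, as is random dodge jumping.
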(event Custom|Moves%20To%20Cover%20And%20Crouch
  ;[1 1 1] Moves to Cover and Crouches
  (if (Variables|Default|GetEnemyDetected)
    (AI|AIMoveTo (Variables|Default|GetAI_Controller_Ref) (Class|BTFunctionLibrary|GetBlackboardValueasVector (Variables|Default|GetCoverMove)) 0 -1.0 "Default" "Default" true true
      (:OnMoveFinished
        (bind _asbase_ai_character (Utilities|Casting|CastToBase_AI_Character (Variables|Default|GetControlled_Pawn_Ref)))
        (Default|EnterCover _asbase_ai_character)
        ;;[1 0.3521 0.4019] When in cover, set to true
        (Class|BTFunctionLibrary|SetBlackboardValueasBool (Variables|Default|GetBB_InCover) true)))))

(event EventReceiveTickAI
  (params (OwnerController :type AI%20Controller%20Object%20Reference) (ControlledPawn :type Pawn%20Object%20Reference) (DeltaSeconds :type Float%20%28single-precision%29))
  ;[0.3355 1 0.8494] Detect Enemies to Shoot
  (Variables|Default|SetAI_Controller_Ref OwnerController)
  (Variables|Default|SetControlled_Pawn_Ref ControlledPawn)
  (Utilities|IsValid (Class|AIController|GetFocusActor (Variables|Default|GetAI_Controller_Ref))
    (:Is%20Valid
      ;;[0.49 1 0.4779] Creates Sphere, based on Radius size, for detecting enemies
      (bind (_outhit _returnvalue) (Collision|SphereTraceByChannel (Transformation|GetActorLocation (Variables|Default|GetControlled_Pawn_Ref)) (Transformation|GetActorLocation (Class|AIController|GetFocusActor (Variables|Default|GetAI_Controller_Ref))) 4.5e+02 "TraceTypeQuery2" false (Utilities|Array|MakeArray (Variables|Default|GetAI%20Calling%20Event)) "None"))
      (if _returnvalue
        ;;[1 0.9438 0.2661] If Hit Actor is in the focus of the AI then shoot
        ;;;[1 0 0.0421] THIS IS FAILING
        (Variables|Default|SetEnemyDetected _returnvalue)
        (bind _asbase_character (Utilities|Casting|CastToBase_Character (.HitActor (Collision|BreakHitResult _outhit))))
        (if (!= (Variables|/Game/COMBAT_EQS_AI/Characters/ParentChar/Base_Character.Base_Character_C|GetTeamTag _asbase_character) (Variables|/Game/COMBAT_EQS_AI/Characters/ParentChar/Base_Character.Base_Character_C|GetTeamTag (Variables|Default|GetAI%20Calling%20Event)))
          (Default|Shoot (Variables|Default|GetAI%20Calling%20Event))
          (else
            (Development|PrintString "Hello")))))))

(event EventReceiveActivationAI
  (params (OwnerController :type AI%20Controller%20Object%20Reference) (ControlledPawn :type Pawn%20Object%20Reference))
  ;[1 0 0.5263] When Activated
  ;;[0 0 0] Creates Reference to Enemy AI Character
  (bind _asbase_ai_character (Utilities|Casting|CastToBase_AI_Character ControlledPawn))
  (Variables|Default|SetAI%20Calling%20Event _asbase_ai_character)
  ;;[0 0 0] Creates Reference To AI Controller
  (Variables|Default|SetOwner%20Controller OwnerController))