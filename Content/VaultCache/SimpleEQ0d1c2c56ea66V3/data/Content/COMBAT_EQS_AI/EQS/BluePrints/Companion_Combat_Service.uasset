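; Behavior Tree service that makes a companion AI shoot enemies, noted as Bravo Team, along its line to the focused actor.
; Each tick a thin sphere trace runs from the pawn to its focus actor.
; A hit becomes the blackboard TargetActor and triggers Shoot on the cached Base_AI_Character.
; Each hit also restarts a short timer that clears the inCombat blackboard flag once shooting stops.
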(event Custom|RunInCombatFalse
  ;[1 0.4062 0.9221] Detects Bravo Team And Shoots Them
  ;;[1 0.8936 0] Waits a certain amount of time before calling the event to set inCombat to False.
  (CallFunction|SetinCombatBoolFalse))

(event Custom|SetInCombatBoolFalse
  (bind _blackboardref (Variables|Default|GetBlackBoardRef))
  ;[1 1 1] Ensures that inCombat is set to FALSE when not shooting. Shooting will set it to true.
  (Utilities|IsValid _blackboardref
    (:Is%20Valid
      (AI|Components|Blackboard|SetValueasBool _blackboardref (Utilities|Name|MakeLiteralName "inCombat") false))))

(event EventReceiveActivationAI
  (params (OwnerController :type AI%20Controller%20Object%20Reference) (ControlledPawn :type Pawn%20Object%20Reference))
  ;[0.5236 0.3904 1] Get Reference To Self On Activation
  (bind _asbase_ai_character (Utilities|Casting|CastToBase_AI_Character ControlledPawn))
  (Variables|Default|SetCompanionControlledAIRef _asbase_ai_character))

(event EventReceiveTickAI
  (params (OwnerController :type AI%20Controller%20Object%20Reference) (ControlledPawn :type Pawn%20Object%20Reference) (DeltaSeconds :type Float%20%28single-precision%29))
  ;[1 0.4062 0.9221] Detects Bravo Team And Shoots Them
  (Variables|Default|SetOwner%20Controller%20Ref OwnerController)
  (Variables|Default|SetControlled%20Pawn%20Ref ControlledPawn)
  (Utilities|IsValid (Class|AIController|GetFocusActor (Variables|Default|GetOwner%20Controller%20Ref))
    (:Is%20Valid
      ;;[0.1382 1 0] Gets Enemy Actor And Sets As BB Target Actor
      (bind (_outhit _returnvalue) (Collision|SphereTraceByChannel (Transformation|GetActorLocation (Variables|Default|GetControlled%20Pawn%20Ref)) (Transformation|GetActorLocation (Class|AIController|GetFocusActor (Variables|Default|GetOwner%20Controller%20Ref))) 5.0 "TraceTypeQuery2" false (Utilities|Array|MakeArray (Variables|Default|GetCompanionControlledAIRef) (Class|GameplayStatics|GetPlayerControllerfromID)) "None"))
      (if _returnvalue
        (Class|BTFunctionLibrary|SetBlackboardValueasObject (Variables|Default|GetTargetActor) (.HitActor (Collision|BreakHitResult _outhit)))
        ;;[1 0.0399 0] Starts To Shoot Enemy
        (Default|Shoot (Variables|Default|GetCompanionControlledAIRef))
        ;;[1 0.8936 0] Waits a certain amount of time before calling the event to set inCombat to False.
        (Utilities|Time|SetTimerbyEvent (delegate Custom|RunInCombatFalse) 2.5)))))