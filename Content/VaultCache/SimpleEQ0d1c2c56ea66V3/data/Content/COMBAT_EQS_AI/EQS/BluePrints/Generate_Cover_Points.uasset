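; EQS generator that produces candidate cover points around the player for AI hiding from the player's visibility.
; It casts a ring of evenly spaced Visibility traces from a set radius inward to the player's navmesh-projected location.
; Each hit's impact point, pushed off the surface along its normal and raised above it, becomes a generated query point.
; The point array is cleared on every generation, and the context locations input is unused.
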(fn DoItemGeneration
  (params (ContextLocations :type Array%20of%20Vectors))
  (bind _returnvalue (Game|GetPlayerCharacter 0))
  (bind _returnvalue_2 (Transformation|GetActorLocation _returnvalue))
  (bind _projectedlocation (AI|Navigation|ProjectPointtoNavigation _returnvalue_2 0 "/Script/NavigationSystem.RecastFilter_UseDefaultArea" "0, 0, 0"))
  ;[0 0.7224 1] All the points that are being fed into the EQS
  ;[0.2309 1 0] Clears array of cover points every time this funciton is called. This prevents lagging and ensures points are valid.
  (Utilities|Array|Clear (Variables|Default|GetLocationSet))
  ;[1 0 0.009362] Generates spokes for line trace. More spokes more accurate. Each spoke is 10 degrees. 36 spokes * 10.
  (for _index (range 0 35)
    (Utilities|IsValid _returnvalue
      (:Is%20Valid
        ;[0.3672 1 0.653] End point will be going into the actor since this is about AI covering from the visibility of other actors
        (bind (_outhit _returnvalue_3) (Collision|LineTraceByChannel (+ (* (Math|Vector|RotateVector "1.000000, 0, 0" (Math|Rotator|MakeRotator 0.0 0.0 (* _index 1e+01))) (Variables|Default|GetRadius)) _projectedlocation) _projectedlocation "TraceTypeQuery1" false 0 "None"))
        ;[0.6871 1 0.1146] Becomes True if return value hits an object
        (if _returnvalue_3
          ;[0.1622 0.4633 1] Adds Impact Point of Line trace to array
          (Utilities|Array|Add (Variables|Default|GetLocationSet) (+ (.ImpactPoint (Collision|BreakHitResult _outhit)) (* (.ImpactNormal (Collision|BreakHitResult _outhit)) 5e+01) "0,0,100.000000"))))))
  ;[0.7354 0.3512 1] Adds location of impact points to vectors to be used within level
  (for _array_element (Variables|Default|GetLocationSet)
    (Class|EnvQueryGeneratorBlueprintBase|AddGeneratedVector _array_element))
  ;[1 1 1] Output Node
  (return))