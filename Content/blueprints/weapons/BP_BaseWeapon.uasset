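; Base weapon Blueprint providing shared ammo and hitscan firing logic, with empty Shoot and EndShoot events.
; It caches the first-person player character at BeginPlay and pushes ammo updates to it.
; CreateShotTrace decrements the magazine first, so reaching zero plays an empty click at world origin instead of firing.
; Otherwise it spawns a muzzle effect and runs a debug-drawn multi-object trace from ShootArrow, applying blood effects and damage to every hit.
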(event Custom|CreateShotTrace
  (params (Range :type Float%20%28double-precision%29))
  (bind _shootarrow (Variables|Default|GetShootArrow))
  (bind _returnvalue (Transformation|GetWorldLocation _shootarrow))
  (bind _output_get (Variables|Default|SetCurrentMagAmmo (Math|Integer|Clamp(Integer) (- (Variables|Default|GetCurrentMagAmmo) 1) 0 (Variables|Default|GetMaxMagAmmo))))
  (Default|UpdateAmmo (Variables|Default|GetPlayerCharacter) _output_get (Variables|Default|GetCurrentReserveAmmo))
  (if (<= _output_get 0)
    (Audio|PlaySoundatLocation "/Game/InterfaceAndItemSounds/WAV/Back_Click_11_wav.Back_Click_11_wav" "0, 0, 0" "0, 0, 0" 1.0 1.0 0.0 0 0 0 0)
    (else
      (Effects|SpawnEmitterAttached "/Game/Realistic_Starter_VFX_Pack_Vol2/Particles/Explosion/P_Explosion_Big_A.P_Explosion_Big_A" _shootarrow "None" "0, 0, 0" "0, 0, 0" "0.020000,0.020000,0.020000")
      (bind (_outhits _returnvalue_2) (Class|KismetSystemLibrary|LineTraceMultiforObjects _returnvalue (+ _returnvalue (* (Math|Vector|GetForwardVector (Transformation|GetWorldRotation _shootarrow)) Range)) (Utilities|Array|MakeArray "ObjectTypeQuery3" "ObjectTypeQuery4") false 0 "ForDuration" true))
      (if _returnvalue_2
        (bind _array_element (Utilities|Array|ForEachLoopwithBreak _outhits)
          (:LoopBody
            (Effects|SpawnEmitteratLocation "/Game/Realistic_Starter_VFX_Pack_Vol2/Particles/Blood/P_Blood_Splat_Cone.P_Blood_Splat_Cone" (.Location (Collision|BreakHitResult _array_element)))
            (Game|Damage|ApplyDamage (.HitActor (Collision|BreakHitResult _array_element)) (Variables|Default|GetDamage) 0 0)))))))

(event Custom|Shoot)

(event Custom|EndShoot)

(event EventBeginPlay
  (bind _asbp_first_person_character (Utilities|Casting|CastToBP_FirstPersonCharacter (Game|GetPlayerCharacter 0)))
  (Variables|Default|SetPlayerCharacter _asbp_first_person_character))

(fn ConstructionScript)