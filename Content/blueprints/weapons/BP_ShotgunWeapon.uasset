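; Shotgun weapon Blueprint that extends a parent weapon's Shoot event with smoke and a rate-limited shot trace.
; Each Shoot call runs the parent logic and attaches a smoke emitter to ShootArrow, even during cooldown.
; When CanShoot is true, it clears the flag, creates one trace over Range and starts a FireRate timer whose ResetShot event re-enables shooting.
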(event Custom|ResetShot
  (Variables|Default|SetCanShoot true))

(event EventShoot
  (|CallParentFunction)
  (Effects|SpawnEmitterAttached "/Game/Realistic_Starter_VFX_Pack_Vol2/Particles/Explosion/P_Explosion_Smoke.P_Explosion_Smoke" (Variables|Default|GetShootArrow) "None")
  (if (Variables|Default|GetCanShoot)
    (Variables|Default|SetCanShoot false)
    (CallFunction|CreateShotTrace (Variables|Default|GetRange))
    (Utilities|Time|SetTimerbyEvent (delegate Custom|ResetShot) (Variables|Default|GetFireRate))))

(fn ConstructionScript
  (|CallParentFunction))