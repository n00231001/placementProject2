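; BP_enemy is a melee enemy that chases the player, attacks on reaching them, and dies when its health runs out.
; PawnSensing sets a seen flag that starts an AI MoveTo toward the player, while Tick halts movement until that flag is set.
; On arrival it plays an attack montage and damages actors in a sphere at its arrow, destroying itself upon any hit.
; AnyDamage reduces Health and destroys it at zero.
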(event OnSeePawn(PawnSensing)
  (params (Pawn :type Pawn%20Object%20Reference))
  (Variables|Default|SetisSeeingPlayer true)
  (CallFunction|FollowPlayer))

(event Custom|FollowPlayer
  (Variables|Default|SetcanAttack true)
  (if (Variables|Default|GetisSeeingPlayer)
    (AI|AIMoveTo self "0, 0, 0" (Game|GetPlayerCharacter 0) 7e+01 false
      (:OnSuccess
        (if (Variables|Default|GetcanAttack)
          (Variables|Default|SetcanAttack false)
          (bind _returnvalue (Animation|PlayAnimMontage "/Game/enemies/attack.attack" 2.0 "None"))
          (bind _outactors (Collision|SphereOverlapActors (Transformation|GetWorldLocation (Variables|Default|GetArrow1)) 1e+02 (Variables|Default|GetObject%20Types) 0))
          (bind _array_element (Utilities|Array|ForEachLoopwithBreak _outactors)
            (:LoopBody
              (Game|Damage|ApplyDamage _array_element 1e+01 0 0)
              (Actor|DestroyActor))
            (:Completed
              (Utilities|FlowControl|Delay _returnvalue)
              (Variables|Default|SetcanAttack true))))))
    (else
      (Variables|Default|SetisSeeingPlayer false))))

(event EventBeginPlay)

(event Collision|EventActorBeginOverlap
  (params (OtherActor :type Actor%20Object%20Reference)))

(event EventTick
  (params (DeltaSeconds :type Float%20%28single-precision%29))
  (if (not (Variables|Default|GetisSeeingPlayer))
    (Components|Movement|StopMovementImmediately (Variables|Character|GetCharacterMovement))))

(event Game|Damage|EventAnyDamage
  (params (Damage :type Float%20%28single-precision%29) (DamageType :type Damage%20Type%20Object%20Reference) (InstigatedBy :type Controller%20Object%20Reference) (DamageCauser :type Actor%20Object%20Reference))
  (bind _output_get (Variables|Default|SetHealth (- (Variables|Default|GetHealth) Damage)))
  (if (<= _output_get 0.0)
    (Utilities|Casting|CastToBP_FirstPersonCharacter (Game|GetPlayerCharacter 0))
    (Actor|DestroyActor)))

(fn ConstructionScript)