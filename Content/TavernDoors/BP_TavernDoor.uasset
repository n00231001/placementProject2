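; BP_TavernDoor is a tavern door actor that swings open when interacted with.
; A sphere trigger shows a widget component when something overlaps it and hides it when the overlap ends.
; The Interact event hides the widget and plays the DoorSwing timeline from the start, lerping the Hinge's relative rotation to a 90-degree yaw.
; It has no closing logic, and the overlap events do not check which actor triggered them.
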(event OnComponentBeginOverlap(Sphere)
  (params (OverlappedComponent :type Primitive%20Component%20Object%20Reference) (OtherActor :type Actor%20Object%20Reference) (OtherComp :type Primitive%20Component%20Object%20Reference) (OtherBodyIndex :type Integer) (bFromSweep :type Boolean) (SweepResult :type Hit%20Result%20Structure%20%28by%20ref%29))
  (Rendering|SetVisibility (Variables|Default|GetWidget) true false))

(event OnComponentEndOverlap(Sphere)
  (params (OverlappedComponent :type Primitive%20Component%20Object%20Reference) (OtherActor :type Actor%20Object%20Reference) (OtherComp :type Primitive%20Component%20Object%20Reference) (OtherBodyIndex :type Integer))
  (Rendering|SetVisibility (Variables|Default|GetWidget) false false))

(event EventBeginPlay)

(event Collision|EventActorBeginOverlap
  (params (OtherActor :type Actor%20Object%20Reference)))

(event EventTick
  (params (DeltaSeconds :type Float%20%28single-precision%29)))

(event EventInteract
  (Rendering|SetVisibility (Variables|Default|GetWidget) false false)
  (bind _newtrack_0 (Timeline|DoorSwing PlayFromStart)
    (:Update
      (Transformation|SetRelativeRotation (Variables|Default|GetHinge) (Math|Rotator|Lerp(Rotator) "0, 0, 0" "0.000000,-90.000000,0.000000" _newtrack_0) false false))))

(fn ConstructionScript)